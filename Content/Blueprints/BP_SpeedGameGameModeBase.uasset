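; Game mode Blueprint for the speed game that relays gameplay data to the in-game HUD.
; Three events push speed (noted as MPH for now), the timer, and highscores with an index for name entry to the widget.
; Each casts CurrentWidget to WB_IngameHUD and calls its matching update function, doing nothing if the cast fails.
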(event `self.UpdateSpeedOnUI`
  (params (speed :type Integer))
  ;[1 1 1] Show current speed on widget in MPH (for now)
  (bind _aswb_ingame_hud (cast `/Game/Blueprints/UI/WB_IngameHUD` (`self.CurrentWidget`)))
  (`/Game/Blueprints/UI/WB_IngameHUD.UpdateSpeedOnUI` _aswb_ingame_hud speed))

(event `self.UpdateTimnerOnUI`
  (params (speed :type "Float (single-precision)"))
  ;[1 1 1] Show ccurernt timer on widget
  (bind _aswb_ingame_hud (cast `/Game/Blueprints/UI/WB_IngameHUD` (`self.CurrentWidget`)))
  (`/Game/Blueprints/UI/WB_IngameHUD.UpdateTimerOnUI` _aswb_ingame_hud speed))

(event `self.ShowHighScoresOnUI`
  (params (highscores :type "Array of HighScoreData Structure (by ref)") (indexToSetName :type Integer))
  ;[1 1 1] Show highscores on screen
  (bind _aswb_ingame_hud (cast `/Game/Blueprints/UI/WB_IngameHUD` (`self.CurrentWidget`)))
  (`/Game/Blueprints/UI/WB_IngameHUD.ShowHighScores` _aswb_ingame_hud highscores indexToSetName))

(fn `UserConstructionScript`)