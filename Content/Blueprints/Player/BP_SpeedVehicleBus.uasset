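; Player bus vehicle for a Speed-style game, driving the audio and visual feedback for a bomb tied to driving speed.
; Tick feeds forward speed into the engine sound's RPM and, while the bomb is active, flickers the body red with timed ticking below 60 mph, escalating below 55.
; An exploded status stops the engine and plays a random blast once.
; An any-key and mouse hack reports gamepad versus keyboard-mouse input to the game mode.
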(event `Key|AnyKey`
  (params (Key :type "Key Structure"))
  (bind _returnvalue (`GameplayStatics.GetGameMode`))
  ;[1 1 1] Hack to find what input is being used
  (:`Pressed`
    (if (`KismetInputLibrary.Key_IsGamepadKey` Key)
      (bind _asbp_speed_game_game_mode_base (cast `/Game/Blueprints/BP_SpeedGameGameModeBase` _returnvalue))
      (`/Game/Blueprints/BP_SpeedGameGameModeBase.SetCurrentInput` _asbp_speed_game_game_mode_base false)
      (else
        (bind _asbp_speed_game_game_mode_base_2 (cast `/Game/Blueprints/BP_SpeedGameGameModeBase` _returnvalue :!label _label))
        (`/Game/Blueprints/BP_SpeedGameGameModeBase.SetCurrentInput` _asbp_speed_game_game_mode_base_2 true)))))

(event `self.ReceiveBeginPlay`
  (bind _mesh (`self.Mesh`))
  (bind _aschaos_wheeled_vehicle_movement_component (cast `ChaosWheeledVehicleMovementComponent` (`self.VehicleMovementComponent`)))
  (set `self.ChaosWheeledVehicleMovementComponent` _aschaos_wheeled_vehicle_movement_component)
  (bind _returnvalue (`PrimitiveComponent.CreateDynamicMaterialInstance` _mesh 0 (`PrimitiveComponent.GetMaterial` _mesh 0) "None"))
  (bind _output_get (set `self.DM_Bus` _returnvalue))
  (bind _returnvalue_2 (`MaterialInstanceDynamic.K2_GetVectorParameterValue` _output_get "CarColor"))
  (set `self.OriginalMeshColor` _returnvalue_2)
  (`AudioComponent.SetVolumeMultiplier` (`self.Bomb`) 0.0))

(event `InputVectorAxis|Mouse2D`
  (params (AxisValue :type "Vector Structure"))
  ;[1 1 1] Hack to find what input is being used
  (if (`KismetMathLibrary.NotEqualExactly_VectorVector` AxisValue (`KismetMathLibrary.Vector_Zero`))
    (goto _label)))

(event `self.ReceiveTick`
  (params (DeltaSeconds :type "Float (single-precision)"))
  (bind _bomb (`self.Bomb`))
  (bind _dm_bus (`self.DM_Bus`))
  (bind _engine (`self.Engine`))
  (bind _returnvalue (`ChaosVehicleMovementComponent.GetForwardSpeedMPH` (`self.VehicleMovementComponent`)))
  (bind _returnvalue_2 (`KismetMathLibrary.MapRangeClamped` (`KismetMathLibrary.Abs` (`ChaosVehicleMovementComponent.GetForwardSpeed` (`self.VehicleMovementComponent`))) 0.0 (`self.MaxRpm`) 0.0 1.0))
  (`|ExecutionSequence`
    (:`then_0`
      ;[1 1 1] Handle sound
      (if (`|EnumEquality` (`self.CurrentBombStatus`) "Explodeded")
        (`/Engine/EditorBlueprintResources/StandardMacros.DoOnce` false
          (:`Completed`
            (`KismetSystemLibrary.K2_ClearAndInvalidateTimerHandle` (`self.bombTimer`))
            (`AudioComponent.Stop` _engine)
            (`GameplayStatics.PlaySoundAtLocation` (`KismetArrayLibrary.Array_Random` (`self.ExplosionSounds`)) (`self.K2_GetActorLocation`) (struct) 1.0 1.0 0.01 "/Game/Sound/Bus/SE_Bus.SE_Bus" null null null)
            (`MaterialInstanceDynamic.SetScalarParameterValue` (`self.DM_Bus`) "IsFlickering" 0.0)
            (`AudioComponent.SetVolumeMultiplier` (`self.Bomb`) 0.0)))
        (else
          (`AudioComponent.SetVolumeMultiplier` _engine 0.5)
          (set `self.CurrentRPMClamped` _returnvalue_2)
          (`AudioComponent.SetFloatParameter` _engine "RPM" _returnvalue_2))))
    (:`then_1`
      ;[1 1 1] If player goes below 60 mph
      (if (`|EnumEquality` (`self.CurrentBombStatus`) "Active")
        (if (<= _returnvalue 60.0)
          (if (<= _returnvalue 55.0)
            (`MaterialInstanceDynamic.SetScalarParameterValue` _dm_bus "FlickerSpeed" 5.0)
            (`AudioComponent.SetVolumeMultiplier` _bomb 1.0)
            (else
              (`MaterialInstanceDynamic.SetScalarParameterValue` _dm_bus "IsFlickering" 1.0)
              (`MaterialInstanceDynamic.SetScalarParameterValue` _dm_bus "FlickerSpeed" 1.0)
              (`MaterialInstanceDynamic.SetVectorParameterValue` _dm_bus "CarColor" (struct :`R` 1.0 :`A` 1.0))
              (`AudioComponent.SetVolumeMultiplier` _bomb 0.0)
              (`/Engine/EditorBlueprintResources/StandardMacros.DoOnce` false :!label _label_2
                (:`Completed`
                  (bind _returnvalue_3 (`KismetSystemLibrary.K2_SetTimerDelegate` (delegate `PlayBombTick`) 1.0 true -1.0))
                  (set `self.bombTimer` _returnvalue_3)))))
          (else
            (`MaterialInstanceDynamic.SetScalarParameterValue` _dm_bus "IsFlickering" 0.0)
            (`MaterialInstanceDynamic.SetVectorParameterValue` _dm_bus "CarColor" (`self.OriginalMeshColor`))
            (`KismetSystemLibrary.K2_ClearAndInvalidateTimerHandle` (`self.bombTimer`))
            (goto _label_2 :!via `Reset`)))))))

(event `PlayBombTick`
  ;[1 1 1] If player goes below 60 mph
  (`GameplayStatics.PlaySoundAtLocation` "/Game/Sound/Bus/ticking.ticking" (`self.K2_GetActorLocation`) (struct) 1.0 1.0 0.01 "/Game/Sound/Bus/SE_Bus.SE_Bus" null null null))

(fn `UserConstructionScript`)