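; Player bus vehicle for the Speed bomb game, handling engine audio, input-type detection and level reload.
; Tick maps absolute forward speed to the engine sound's RPM parameter, or, once the bomb has exploded, stops it and plays a random explosion sound once.
; A stopgap input check records the device type, though every branch currently sets Keyboard.
; Escape reloads the level through the game instance only while bomb status is None.
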(event `self.ReceiveBeginPlay`
  (bind _aschaos_wheeled_vehicle_movement_component (cast `ChaosWheeledVehicleMovementComponent` (`self.VehicleMovementComponent`)))
  (set `self.ChaosWheeledVehicleMovementComponent` _aschaos_wheeled_vehicle_movement_component))

(event `Key|AnyKey`
  (params (Key :type "Key Structure"))
  ;[1 1 1] Hack to find what input is being used - put this in game controller tbh
  (:`Pressed`
    (if (`KismetInputLibrary.Key_IsGamepadKey` Key)
      (set `self.CurrentInputType` "Keyboard")
      (else
        (set `self.CurrentInputType` "Keyboard" :!label _label)))))

(event `InputVectorAxis|Mouse2D`
  (params (AxisValue :type "Vector Structure"))
  ;[1 1 1] Hack to find what input is being used - put this in game controller tbh
  (if (`KismetMathLibrary.NotEqualExactly_VectorVector` AxisValue (`KismetMathLibrary.Vector_Zero`))
    (goto _label)))

(event `self.ReceiveTick`
  (params (DeltaSeconds :type "Float (single-precision)"))
  (bind _engine (`self.Engine`))
  (bind _returnvalue (`KismetMathLibrary.MapRangeClamped` (`KismetMathLibrary.Abs` (`ChaosVehicleMovementComponent.GetForwardSpeed` (`self.VehicleMovementComponent`))) 0.0 (`self.MaxRpm`) 0.0 1.0))
  (`|ExecutionSequence`
    (:`then_0`
      ;[1 1 1] Handle sound
      (if (`|EnumEquality` (`self.CurrentBombStatus`) "Explodeded")
        (`/Engine/EditorBlueprintResources/StandardMacros.DoOnce` false
          (:`Completed`
            (`AudioComponent.Stop` _engine)
            (`GameplayStatics.PlaySoundAtLocation` (`KismetArrayLibrary.Array_Random` (`self.ExplosionSounds`)) (`self.K2_GetActorLocation`) (struct) 1.0 1.0 0.01 "/Game/Sound/Bus/SE_Bus.SE_Bus" null null null)))
        (else
          (`AudioComponent.SetVolumeMultiplier` _engine 0.5)
          (set `self.CurrentRPMClamped` _returnvalue)
          (`AudioComponent.SetFloatParameter` _engine "RPM" _returnvalue))))))

(event `Key|Escape`
  (params (Key :type "Key Structure"))
  (:`Pressed`
    (if (`|EnumEquality` (`self.CurrentBombStatus`))
      (bind _asbp_speed_game_instance (cast `/Game/Blueprints/BP_SpeedGameInstance` (`GameplayStatics.GetGameInstance`)))
      (`/Game/Blueprints/BP_SpeedGameInstance.ReloadLevel` _asbp_speed_game_instance))))

(fn `UserConstructionScript`)