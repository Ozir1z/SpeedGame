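; Road spawner actor serving as the start area and drive-over menu of a bus speed game.
; Driving the bus into the start box starts the game and initializes the bus and RoadGenerator, then hides the area.
; Holding the bus on the trial-track trigger toggles the trial track after color and flicker warnings.
; High score and settings triggers show widgets and re-attach the bus camera, with saved scores and road color loaded on BeginPlay.
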(event `self.StartBox.OnComponentBeginOverlap`
  (params (OverlappedComponent :type "PrimitiveComponent Object Reference") (OtherActor :type "Actor Object Reference") (OtherComp :type "PrimitiveComponent Object Reference") (OtherBodyIndex :type Integer) (bFromSweep :type Boolean) (SweepResult :type "HitResult Structure (by ref)"))
  ;[1 1 1] Begin the game
  (bind _asbp_speed_vehicle_bus (cast `/Game/Blueprints/Player/BP_SpeedVehicleBus` OtherActor))
  (bind _asbp_speed_game_game_mode_base (cast `/Game/Blueprints/BP_SpeedGameGameModeBase` (`GameplayStatics.GetGameMode`)))
  (`/Game/Blueprints/BP_SpeedGameGameModeBase.StartGame` _asbp_speed_game_game_mode_base)
  (`SpeedVehiclePawn.Init` _asbp_speed_vehicle_bus)
  (`RoadGenerator.Init` (`self.RoadGenerator`))
  (`KismetSystemLibrary.Delay` 5.0)
  (`self.K2_AddActorLocalOffset` (0.0 0.0 100.0))
  (`KismetSystemLibrary.Delay` 0.1)
  (`SceneComponent.SetVisibility` (`self.DefaultSceneRoot`) false true))

(event `self.TrialTrackTrigger.OnComponentBeginOverlap`
  (params (OverlappedComponent :type "PrimitiveComponent Object Reference") (OtherActor :type "Actor Object Reference") (OtherComp :type "PrimitiveComponent Object Reference") (OtherBodyIndex :type Integer) (bFromSweep :type Boolean) (SweepResult :type "HitResult Structure (by ref)"))
  (bind _dmi_trialtracktrigger (`self.DMI_TrialTrackTrigger`))
  (bind _dmi_trialtracktrigger_2 (`self.DMI_TrialTrackTrigger`))
  ;[1 1 1] Handle Trial Track overlap... THIS IS FUCKING GROSS ROB, PUT IT IN CODE
  (cast `/Game/Blueprints/Player/BP_SpeedVehicleBus` OtherActor)
  (if (`self.TrialTrackExists`)
    (if (not (`self.TrialTrackIsBeingDeleted`))
      (set `self.TrialTrackIsBeingDeleted` true)
      (`MaterialInstanceDynamic.SetVectorParameterValue` _dmi_trialtracktrigger_2 "BaseColor" (`KismetMathLibrary.LinearColor_Red`))
      (`KismetSystemLibrary.Delay` 1.0)
      (if (`self.TrialTrackIsBeingDeleted`)
        (`MaterialInstanceDynamic.SetScalarParameterValue` _dmi_trialtracktrigger_2 "IsFlickering" 1.0)
        (`KismetSystemLibrary.Delay` 5.0)
        (if (`self.TrialTrackIsBeingDeleted`)
          (`MaterialInstanceDynamic.SetScalarParameterValue` _dmi_trialtracktrigger_2 "IsFlickering" 0.0)
          (`RoadGenerator.DeleteTrialTrack` (`self.RoadGenerator`))
          (set `self.TrialTrackIsBeingDeleted` false)
          (set `self.TrialTrackExists` false))))
    (elif (not (`self.TrialTrackIsBeingAdded`))
      (set `self.TrialTrackIsBeingAdded` true)
      (`MaterialInstanceDynamic.SetVectorParameterValue` _dmi_trialtracktrigger "BaseColor" (`KismetMathLibrary.LinearColor_Green`))
      (`KismetSystemLibrary.Delay` 1.0)
      (if (`self.TrialTrackIsBeingAdded`)
        (`MaterialInstanceDynamic.SetScalarParameterValue` _dmi_trialtracktrigger "IsFlickering" 1.0)
        (`KismetSystemLibrary.Delay` 5.0)
        (if (`self.TrialTrackIsBeingAdded`)
          (`MaterialInstanceDynamic.SetScalarParameterValue` _dmi_trialtracktrigger "IsFlickering" 0.0)
          (`RoadGenerator.GenerateTrialTrack` (`self.RoadGenerator`))
          (set `self.TrialTrackIsBeingAdded` false)
          (set `self.TrialTrackExists` true))))))

(event `self.TrialTrackTrigger.OnComponentEndOverlap`
  (params (OverlappedComponent :type "PrimitiveComponent Object Reference") (OtherActor :type "Actor Object Reference") (OtherComp :type "PrimitiveComponent Object Reference") (OtherBodyIndex :type Integer))
  (bind _trialtrackisbeingadded (`self.TrialTrackIsBeingAdded`))
  (bind _trialtrackisbeingdeleted (`self.TrialTrackIsBeingDeleted`))
  ;[1 1 1] Handle Trial Track overlap... THIS IS FUCKING GROSS ROB, PUT IT IN CODE
  (if (or _trialtrackisbeingdeleted _trialtrackisbeingadded)
    (set `self.TrialTrackIsBeingDeleted` false)
    (set `self.TrialTrackIsBeingAdded` false)
    (cast `/Game/Blueprints/Player/BP_SpeedVehicleBus` OtherActor :!label _label)
    (`MaterialInstanceDynamic.SetVectorParameterValue` (`self.DMI_TrialTrackTrigger`) "BaseColor" (`self.Color_TriggerOrignal`))
    (`MaterialInstanceDynamic.SetScalarParameterValue` (`self.DMI_TrialTrackTrigger`) "IsFlickering" 0.0)
    (elif _trialtrackisbeingdeleted
      _
      (elif (not _trialtrackisbeingadded)
        (goto _label)))))

(event `self.ReceiveBeginPlay`
  (bind _returnvalue (`SpeedGameUserSettings.GetSpeedGameUserSettings`))
  (bind _settingstrigger (`self.SettingsTrigger`))
  (bind _highscoretrigger (`self.HighScoreTrigger`))
  (bind _staticmesh (`self.StaticMesh`))
  (bind _trialtracktrigger (`self.TrialTrackTrigger`))
  (`|ExecutionSequence`
    (:`then_0`
      ;[1 1 1] Create Dynamic Material instances
      (bind _returnvalue_2 (`PrimitiveComponent.CreateDynamicMaterialInstance` _trialtracktrigger 0 (`PrimitiveComponent.GetMaterial` _trialtracktrigger 0) "None"))
      (bind _output_get (set `self.DMI_TrialTrackTrigger` _returnvalue_2))
      (bind _returnvalue_3 (`PrimitiveComponent.CreateDynamicMaterialInstance` _highscoretrigger 0 (`PrimitiveComponent.GetMaterial` _highscoretrigger 0) "None"))
      (set `self.DMI_HighScoreTrigger` _returnvalue_3)
      (bind _returnvalue_4 (`PrimitiveComponent.CreateDynamicMaterialInstance` _settingstrigger 0 (`PrimitiveComponent.GetMaterial` _settingstrigger 0) "None"))
      (set `self.DMI_SettingsTrigger` _returnvalue_4)
      (bind _returnvalue_5 (`PrimitiveComponent.CreateDynamicMaterialInstance` _staticmesh 0 (`PrimitiveComponent.GetMaterial` _staticmesh 0) "None"))
      (set `self.DMI_StartRoadMesh` _returnvalue_5)
      (bind _returnvalue_6 (`MaterialInstanceDynamic.K2_GetVectorParameterValue` _output_get "BaseColor"))
      (set `self.Color_TriggerOrignal` _returnvalue_6))
    (:`then_1`
      ;[1 1 1] Load highscores to highscore UI - and hide
      (bind _aswb_high_score_ui (cast `/Game/Blueprints/UI/WB_HighScoreUI` (`WidgetComponent.GetWidget` (`self.HighScoreUI`))))
      (set `self.WB_HighScoreUI` _aswb_high_score_ui)
      (bind _asbp_speed_game_instance (cast `/Game/Blueprints/BP_SpeedGameInstance` (`GameplayStatics.GetGameInstance`)))
      (`SpeedGameInstance.LoadGame` _asbp_speed_game_instance)
      (`/Game/Blueprints/UI/WB_HighScoreUI.AddHighScores` _aswb_high_score_ui (`SpeedSaveGame.HighScores` (`SpeedGameInstance.SaveGameObject` _asbp_speed_game_instance)))
      (`Widget.SetVisibility` _aswb_high_score_ui "Hidden"))
    (:`then_2`
      ;[1 1 1] Set settings UI and hide
      (bind _aswb_color_settings (cast `/Game/Blueprints/UI/WB_ColorSettings` (`WidgetComponent.GetWidget` (`self.SettingsUI`))))
      (bind _output_get_2 (set `self.WB_SettingsUI` _aswb_color_settings))
      (`/Game/Blueprints/UI/WB_ColorSettings.Init` _output_get_2)
      (`Widget.SetVisibility` _output_get_2 "Hidden")
      (bind _asbp_speed_game_game_mode_base (cast `/Game/Blueprints/BP_SpeedGameGameModeBase` (`GameplayStatics.GetGameMode`)))
      (`GameUserSettings.LoadSettings` _returnvalue false)
      (`MaterialInstanceDynamic.SetVectorParameterValue` (`self.DMI_StartRoadMesh`) "LineColor" (`SpeedGameUserSettings.GetRoadColor` _returnvalue))
      (`/Game/Blueprints/BP_SpeedGameGameModeBase.SetRoadSpawnerAndInitalRoadColor` _asbp_speed_game_game_mode_base self))))

(event `UpdateTrialTrack`
  (params (newColor :type "LinearColor Structure"))
  (`RoadGenerator.UpdateTrialTrack` (`self.RoadGenerator`) newColor))

(event `self.HighScoreTrigger.OnComponentBeginOverlap`
  (params (OverlappedComponent :type "PrimitiveComponent Object Reference") (OtherActor :type "Actor Object Reference") (OtherComp :type "PrimitiveComponent Object Reference") (OtherBodyIndex :type Integer) (bFromSweep :type Boolean) (SweepResult :type "HitResult Structure (by ref)"))
  ;[1 1 1] Handle Highscore menu when driving over trigger
  (`self.Set Visibility` (`KismetMathLibrary.LinearColor_Yellow`) "Visible" (`self.DMI_HighScoreTrigger`) (`self.WB_HighScoreUI`) OtherActor)
  (bind _asbp_speed_vehicle_bus (cast `/Game/Blueprints/Player/BP_SpeedVehicleBus` OtherActor))
  (bind _cameraarmcomp (`SpeedVehiclePawn.CameraArmComp` _asbp_speed_vehicle_bus))
  (set `SpringArmComponent.TargetArmLength` 1500.0 _cameraarmcomp)
  (`SceneComponent.K2_AttachToComponent` _cameraarmcomp (`self.HighscoreCameraPoint`) "None" "SnapToTarget" "SnapToTarget" "KeepRelative" true))

(event `self.SettingsTrigger.OnComponentBeginOverlap`
  (params (OverlappedComponent :type "PrimitiveComponent Object Reference") (OtherActor :type "Actor Object Reference") (OtherComp :type "PrimitiveComponent Object Reference") (OtherBodyIndex :type Integer) (bFromSweep :type Boolean) (SweepResult :type "HitResult Structure (by ref)"))
  (bind _wb_settingsui (`self.WB_SettingsUI`))
  ;[1 1 1] Handle color settings menu when driving over trigger
  (`self.Set Visibility` (`KismetMathLibrary.LinearColor_Yellow`) "Visible" (`self.DMI_SettingsTrigger`) _wb_settingsui OtherActor)
  (`/Game/Blueprints/UI/WB_ColorSettings.SetFocusColorPicker` _wb_settingsui)
  (bind _asbp_speed_vehicle_bus (cast `/Game/Blueprints/Player/BP_SpeedVehicleBus` OtherActor))
  (bind _vehiclemovementcomponent (`WheeledVehiclePawn.VehicleMovementComponent` _asbp_speed_vehicle_bus))
  (`ChaosVehicleMovementComponent.SetThrottleInput` _vehiclemovementcomponent 0.0)
  (`ChaosVehicleMovementComponent.SetHandbrakeInput` _vehiclemovementcomponent true)
  (bind _cameraarmcomp (`SpeedVehiclePawn.CameraArmComp` _asbp_speed_vehicle_bus))
  (set `SpringArmComponent.TargetArmLength` 1500.0 _cameraarmcomp)
  (`SceneComponent.K2_AttachToComponent` _cameraarmcomp (`self.SettingsCameraPoint`) "None" "SnapToTarget" "SnapToTarget" "KeepRelative" true))

(event `self.HighScoreTrigger.OnComponentEndOverlap`
  (params (OverlappedComponent :type "PrimitiveComponent Object Reference") (OtherActor :type "Actor Object Reference") (OtherComp :type "PrimitiveComponent Object Reference") (OtherBodyIndex :type Integer))
  ;[1 1 1] Handle Highscore menu when driving over trigger
  (`self.Set Visibility` (`self.Color_TriggerOrignal`) "Hidden" (`self.DMI_HighScoreTrigger`) (`self.WB_HighScoreUI`) OtherActor)
  (bind _asbp_speed_vehicle_bus (cast `/Game/Blueprints/Player/BP_SpeedVehicleBus` OtherActor))
  (`ChaosVehicleMovementComponent.SetHandbrakeInput` (`WheeledVehiclePawn.VehicleMovementComponent` _asbp_speed_vehicle_bus) false)
  (`SceneComponent.K2_AttachToComponent` (`SpeedVehiclePawn.CameraArmComp` _asbp_speed_vehicle_bus) (`Actor.RootComponent` _asbp_speed_vehicle_bus) "None" "SnapToTarget" "SnapToTarget" "KeepRelative" true))

(event `self.SettingsTrigger.OnComponentEndOverlap`
  (params (OverlappedComponent :type "PrimitiveComponent Object Reference") (OtherActor :type "Actor Object Reference") (OtherComp :type "PrimitiveComponent Object Reference") (OtherBodyIndex :type Integer))
  ;[1 1 1] Handle color settings menu when driving over trigger
  (`self.Set Visibility` (`self.Color_TriggerOrignal`) "Hidden" (`self.DMI_SettingsTrigger`) (`self.WB_SettingsUI`) OtherActor)
  (bind _asbp_speed_vehicle_bus (cast `/Game/Blueprints/Player/BP_SpeedVehicleBus` OtherActor))
  (`ChaosVehicleMovementComponent.SetHandbrakeInput` (`WheeledVehiclePawn.VehicleMovementComponent` _asbp_speed_vehicle_bus) false)
  (`SceneComponent.K2_AttachToComponent` (`SpeedVehiclePawn.CameraArmComp` _asbp_speed_vehicle_bus) (`Actor.RootComponent` _asbp_speed_vehicle_bus) "None" "SnapToTarget" "SnapToTarget" "KeepRelative" true))

(fn `Set Visibility`
  (params (colorToChangeTo :type "LinearColor Structure") (VisibilityStatus :type "ESlateVisibility Enum" :default "Visible") (MaterialInstance :type "MaterialInstanceDynamic Object Reference") (UserWidget :type "UserWidget Object Reference") (BusActor :type "Actor Object Reference") (CameraStatus :type "CameraStatus Enum" :default "Follow"))
  (bind _asbp_speed_vehicle_bus (cast `/Game/Blueprints/Player/BP_SpeedVehicleBus` BusActor))
  (`SpeedVehiclePawn.SwitchCameraStatusTo` _asbp_speed_vehicle_bus CameraStatus)
  (`Widget.SetVisibility` UserWidget VisibilityStatus)
  (`MaterialInstanceDynamic.SetVectorParameterValue` MaterialInstance "BaseColor" colorToChangeTo)
  (return))

(fn `UserConstructionScript`)