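; BP_AIWheeledVehiclePawn is an AI wheeled vehicle pawn that handles car color and engine audio.
; The construction script creates a dynamic material instance, which ChangeColor tints according to the car type, from Slow to Insane.
; Tick maps absolute forward speed to the engine's RPM parameter with slight random pitch variation, or fades the sound out once when dying.
; EndPlay plays an attenuated death sound at the car's location.
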(event `self.ChangeColor`
  (switch `CarType` (`self.CurrentCarType`)
    (:`Slow`
      (set `self.CurrentColor` (`KismetMathLibrary.MakeColor` 1.0 0.0 0.5)))
    (:`Normal`
      (set `self.CurrentColor` (`KismetMathLibrary.MakeColor` 1.0 0.6)))
    (:`Fast`
      (set `self.CurrentColor` (`KismetMathLibrary.MakeColor` 0.0 0.9 0.7)))
    (:`Insane`
      (set `self.CurrentColor` (`KismetMathLibrary.MakeColor` 1.0))))
  (`MaterialInstanceDynamic.SetVectorParameterValue` (`self.DynamicMaterial`) "CarColor" (`self.CurrentColor`)))

(event `self.ReceiveTick`
  (params (DeltaSeconds :type "Float (single-precision)"))
  (bind _engine (`self.Engine`))
  (bind _engine_2 (`self.Engine`))
  (if (`|EnumEquality` (`self.CurrentCarStatus`) "Dying")
    (`/Engine/EditorBlueprintResources/StandardMacros.DoOnce` false
      (:`Completed`
        (`AudioComponent.FadeOut` _engine_2 1.0 0.0 "Linear")))
    (else
      (`AudioComponent.SetVolumeMultiplier` _engine_2 0.2)
      (set `self.CurrentRPMClamped` (`KismetMathLibrary.MapRangeClamped` (`KismetMathLibrary.Abs` (`ChaosVehicleMovementComponent.GetForwardSpeed` (`self.VehicleMovementComponent`))) 0.0 (`self.MaxRpm`) 0.0 1.0))
      (`AudioComponent.SetPitchMultiplier` _engine (`KismetMathLibrary.RandomFloatInRange` 0.9 1.0))
      (`AudioParameterControllerInterface.SetFloatParameter` _engine "RPM" (`self.CurrentRPMClamped`)))))

(event `self.ReceiveEndPlay`
  (params (EndPlayReason :type "EEndPlayReason Enum" :default "Destroyed"))
  (`GameplayStatics.PlaySoundAtLocation` "/Game/Sound/Car/car_death.car_death" (`self.K2_GetActorLocation`) (struct) 1.0 1.0 0.0 "/Game/Sound/Car/SE_CarDeath.SE_CarDeath" null null null))

(fn `UserConstructionScript`
  (bind _returnvalue (`PrimitiveComponent.CreateDynamicMaterialInstance` (`self.Mesh`) 0 null "None"))
  (set `self.DynamicMaterial` _returnvalue))